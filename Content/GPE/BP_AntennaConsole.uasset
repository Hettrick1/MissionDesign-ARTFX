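; BP_AntennaConsole is an interactable console with a widget progress display that advances a quest and switches the HQ into its lockdown level.
; React enables interaction, reveals the widget, starts its progression and polls for completion on a looping timer.
; Each Interact speeds up the progress through the widget.
; On completion, a DoOnce updates the quest step, unloads the normal HQ stream level and loads the lockdown one.
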(event Custom|CheckProgress
  (if (Variables|/Game/UI/WBP_AntennaConsole.WBP_AntennaConsole_C|GetprogessFinished (stale EventReact _aswbp_antenna_console))
    (Utilities|FlowControl|DoOnce false
      (:Completed
        (Default|UpdateQuestStep (Variables|Default|GetplayerStateRef) 1 3 true 8)
        (Class|GameplayStatics|UnloadStreamLevelbySoftObjectPtr "/Game/Levels/Sublevels/LVL_HQ_1Normal.LVL_HQ_1Normal" false)
        (Class|GameplayStatics|LoadStreamLevelbySoftObjectPtr "/Game/Levels/Sublevels/LVL_HQ_2Lockdown.LVL_HQ_2Lockdown" true false)))))

(event EventReact
  (Variables|Default|SetcanInterract true)
  (Development|SetHiddeninGame (Variables|Default|GetWidget) false false)
  (bind _aswbp_antenna_console (Utilities|Casting|CastToWBP_AntennaConsole (UserInterface|GetWidget (Variables|Default|GetWidget))))
  (Default|IntitiateProgression _aswbp_antenna_console)
  (Utilities|Time|SetTimerbyEvent (delegate Custom|CheckProgress) 0.5 true))

(event EventInteract
  (|CallParentFunction)
  (bind _aswbp_antenna_console (Utilities|Casting|CastToWBP_AntennaConsole (UserInterface|GetWidget (Variables|Default|GetWidget))))
  (Default|FasterProgress _aswbp_antenna_console))

(fn ConstructionScript
  (|CallParentFunction))