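; Trigger volume actor that shows a dialogue message on the first player's HUD when its box is overlapped, then destroys itself.
; The overlap passes DialogueIndex to the HUD without checking which actor entered.
; The construction script uses that index to look up a DT_Dialogues row by position and copy its DialogueTitle.
; It also clamps out-of-range indices, with -1 labelled as no dialogue.
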(event OnComponentBeginOverlap(Box)
  (params (OverlappedComponent :type Primitive%20Component%20Object%20Reference) (OtherActor :type Actor%20Object%20Reference) (OtherComp :type Primitive%20Component%20Object%20Reference) (OtherBodyIndex :type Integer) (bFromSweep :type Boolean) (SweepResult :type Hit%20Result%20Structure%20%28by%20ref%29))
  (Class|BPIHUD|ShowDialogue(Message) (HUD|GetHUD (Game|GetPlayerController 0)) (Variables|Dialogue|GetdialogueIndex))
  (Actor|DestroyActor))

(fn ConstructionScript
  (bind _outrownames (DataTable|GetDataTableRowNames "/Game/DataAssets/Dialogues/DT_Dialogues.DT_Dialogues"))
  (bind _returnvalue (Utilities|GetDataTableRow "/Game/DataAssets/Dialogues/DT_Dialogues.DT_Dialogues" (Utilities|Array|Get(acopy) _outrownames (Variables|Dialogue|GetdialogueIndex)))
    (:then
      (Variables|Dialogue|SetdialogueTitle (.dialogueTitle (Utilities|Struct|BreakS_Dialogues _returnvalue)))
      (Variables|Dialogue|SetdialogueIndex (Math|Integer|Clamp(Integer) (Variables|Dialogue|GetdialogueIndex) -1 (Utilities|Array|LastIndex _outrownames)) :!label _label))
    (:RowNotFound
      (if (== (Variables|Dialogue|GetdialogueIndex) -1)
        (Variables|Dialogue|SetdialogueTitle "no dialogue")
        (else
          (goto _label))))))