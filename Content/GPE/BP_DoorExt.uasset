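; Interactive door actor that toggles open and closed when its SelfReact event fires and CanBeUsed is true.
; A Lerp timeline, with Speed as play rate, swings the Cube 90 degrees in yaw from the start rotation and reverses to close.
; When an actor implementing BPI_Player begins overlapping the Box of an open door, a retriggerable delay closes it after DelayBeforeClosing.
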(event OnComponentBeginOverlap(Box)
  (params (OverlappedComponent :type Primitive%20Component%20Object%20Reference) (OtherActor :type Actor%20Object%20Reference) (OtherComp :type Primitive%20Component%20Object%20Reference) (OtherBodyIndex :type Integer) (bFromSweep :type Boolean) (SweepResult :type Hit%20Result%20Structure%20%28by%20ref%29))
  (if (Utilities|DoesObjectImplementInterface OtherActor "/Game/FirstPerson/Blueprints/Interface/BPI_Player.BPI_Player_C")
    (if (Variables|Default|Getopened)
      (Utilities|FlowControl|RetriggerableDelay (Variables|Default|GetdelayBeforeClosing))
      (CallFunction|CloseDoor))))

(event Custom|OpenDoor
  (bind _startrotation (Variables|Default|GetstartRotation))
  (Variables|Default|Setopened true)
  (bind _alpha (Timeline|Lerp Play)
    (:Update
      (Transformation|SetWorldRotation (Variables|Default|GetCube) (Math|Rotator|Lerp(Rotator) _startrotation (Math|Rotator|MakeRotator 0.0 0.0 (+ (.Yaw (Math|Rotator|BreakRotator _startrotation)) 9e+01)) _alpha) false true))))

(event Custom|CloseDoor
  (bind _startrotation (Variables|Default|GetstartRotation))
  (Variables|Default|Setopened false)
  (bind _alpha (Timeline|Lerp Reverse)
    (:Update
      (Transformation|SetWorldRotation (Variables|Default|GetCube) (Math|Rotator|Lerp(Rotator) _startrotation (Math|Rotator|MakeRotator 0.0 0.0 (+ (.Yaw (Math|Rotator|BreakRotator _startrotation)) 9e+01)) _alpha) false true))))

(event EventBeginPlay
  (Variables|Default|SetstartRotation (Transformation|GetActorRotation))
  (Components|Timeline|SetPlayRate (Variables|Default|GetLerp) (Variables|Default|Getspeed)))

(event EventSelfReact
  (|CallParentFunction)
  (if (Variables|Default|GetcanBeUsed)
    (if (Variables|Default|Getopened)
      (CallFunction|CloseDoor)
      (else
        (CallFunction|OpenDoor)))))

(fn ConstructionScript)