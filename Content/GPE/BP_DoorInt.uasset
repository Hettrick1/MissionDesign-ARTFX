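; BP_DoorInt is a sliding door that toggles open or closed when its React event fires.
; A timeline moves the mesh from the actor's start location along OpenDirection, scaled by mesh bounds radius and OpenFactor, and reverses to close.
; A player entering the box while the door is open starts a retriggerable delay before auto-closing.
; The mesh is configurable via the construction script, and Speed adjusts the timeline play rate.
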(event OnComponentBeginOverlap(Box)
  (params (OverlappedComponent :type Primitive%20Component%20Object%20Reference) (OtherActor :type Actor%20Object%20Reference) (OtherComp :type Primitive%20Component%20Object%20Reference) (OtherBodyIndex :type Integer) (bFromSweep :type Boolean) (SweepResult :type Hit%20Result%20Structure%20%28by%20ref%29))
  (if (Utilities|DoesObjectImplementInterface OtherActor "/Game/FirstPerson/Blueprints/Interface/BPI_Player.BPI_Player_C")
    (if (Variables|Default|Getopened)
      (Utilities|FlowControl|RetriggerableDelay (Variables|Default|GetdelayBeforeClosing))
      (CallFunction|CloseDoor))))

(event Custom|CloseDoor
  (Variables|Default|Setopened false)
  (bind _alpha (Timeline|Lerp Reverse)
    (:Update
      (Transformation|SetWorldLocation (Variables|Default|GetStaticMesh) (Math|Vector|Lerp(Vector) (Variables|Default|GetstartLocation) (+ (* (Variables|Default|GetopenDirection) (* (.SphereRadius (Collision|GetComponentBounds (Variables|Default|GetStaticMesh))) (Variables|Default|GetopenFactor))) (Variables|Default|GetstartLocation)) _alpha) false false))))

(event Custom|OpenDoor
  (Variables|Default|Setopened true)
  (bind _alpha (Timeline|Lerp Play)
    (:Update
      (Transformation|SetWorldLocation (Variables|Default|GetStaticMesh) (Math|Vector|Lerp(Vector) (Variables|Default|GetstartLocation) (+ (* (Variables|Default|GetopenDirection) (* (.SphereRadius (Collision|GetComponentBounds (Variables|Default|GetStaticMesh))) (Variables|Default|GetopenFactor))) (Variables|Default|GetstartLocation)) _alpha) false false))))

(event EventReact
  (if (Variables|Default|Getopened)
    (CallFunction|CloseDoor)
    (else
      (CallFunction|OpenDoor))))

(event EventBeginPlay
  (Variables|Default|SetstartLocation (Transformation|GetActorLocation))
  (Components|Timeline|SetPlayRate (Variables|Default|GetLerp) (- 1.0 (/ 1.0 (Variables|Default|Getspeed)))))

(fn ConstructionScript
  (Components|StaticMesh|SetStaticMesh (Variables|Default|GetStaticMesh) (Variables|Default|Getmesh)))