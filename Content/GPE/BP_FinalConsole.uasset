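; BP_FinalConsole is a console gameplay element that plays the final sequence when it reacts.
; SelfReact runs the parent reaction, plays FinalSequence and sets its WBP_SecurityModule widget inactive.
; If the player state's StepIndex is at least 3, it then unloads the Normal and Lockdown HQ sublevels and streams in SecurityProtocole without blocking.
; A separate TurnOff event swaps the mesh's screen material to the terminal-off look.
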(event Custom|TurnOff
  (Rendering|Material|SetMaterial (Variables|Default|GetCube) 2 "/Game/Assets/Meshes/Database/Console/T_TerminalOff.T_TerminalOff"))

(event EventSelfReact
  (|CallParentFunction)
  (Sequencer|Player|Play (Variables|/Script/LevelSequence.LevelSequenceActor|GetSequencePlayer (Variables|Default|GetFinalSequence)) :!class /Script/MovieScene.MovieSceneSequencePlayer)
  (bind _aswbp_security_module (Utilities|Casting|CastToWBP_SecurityModule (UserInterface|GetWidget (Variables|Default|GetWidget))))
  (Default|SetInactive _aswbp_security_module)
  (if (>= (Variables|/Game/Manager/PS_InGame.PS_InGame_C|GetstepIndex (Variables|Default|GetplayerStateRef)) 3)
    (Class|GameplayStatics|UnloadStreamLevelbySoftObjectPtr "/Game/Levels/Sublevels/LVL_HQ_1Normal.LVL_HQ_1Normal" false)
    (Class|GameplayStatics|UnloadStreamLevelbySoftObjectPtr "/Game/Levels/Sublevels/LVL_HQ_2Lockdown.LVL_HQ_2Lockdown" false)
    (Class|GameplayStatics|LoadStreamLevelbySoftObjectPtr "/Game/Levels/Sublevels/LVL_HQ_3SecurityProtocole.LVL_HQ_3SecurityProtocole" true false)))

(fn ConstructionScript
  (|CallParentFunction))