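; Base Blueprint for interactable objects, which highlight through custom depth stencil and a HUD crosshair change.
; Interact checks required inventory items, optionally consumes them, then runs InteractReaction, which can disable further interaction.
; The reaction notifies linked ReactObjects through BPI_Interact and calls SelfReact if none are linked or flagged.
; Overridable SelfReact starts or advances quests and, when a quest is set, can show dialogue.
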(event Custom|InteractReaction
  ;[1 1 1] Interact Reaction logic
  (Utilities|FlowControl|Sequence
    (:then_0
      (if (Utilities|Array|IsNotEmpty (Variables|Default|GetreactObjects))
        (for _array_element (Variables|Default|GetreactObjects)
          (if (Utilities|DoesObjectImplementInterface _array_element "/Game/FirstPerson/Blueprints/Interface/BPI_Interact.BPI_Interact_C")
            (Class|BPIInteract|React(Message) _array_element)))
        (if (Variables|Default|GetselfReactAswell)
          (CallFunction|SelfReact))
        (else
          (CallFunction|SelfReact))))
    (:then_1
      (Variables|Default|SetcanInterract (not (Variables|Default|GetinteractOnce))))))

(event Custom|SelfReact
  (bind _questinfos (Variables|Default|GetquestInfos))
  ;[1 0.7462 0] Override this event if you want it to be called when the obect is interacted
  (if (!= (.questindex (Variables|Default|GetquestInfos)) -1)
    (bind _asps_in_game (Utilities|Casting|CastToPS_InGame (Game|GetPlayerState 0)))
    (if (.newquest _questinfos)
      (Default|StartQuest _asps_in_game (.questindex _questinfos))
      (else
        (Default|UpdateQuestStep _asps_in_game (.questindex _questinfos) (.stepindex _questinfos) true -1)))
    (if (!= (Variables|Default|GetdialogueIndex) -1)
      (Class|BPIHUD|ShowDialogue(Message) (HUD|GetHUD (Game|GetPlayerController 0)) (Variables|Default|GetdialogueIndex)))))

(event EventInteract
  ;[1 1 1] Interact logic
  (if (Variables|Default|GetcanInterract)
    (if (and (Variables|Default|GetneedItem) (Utilities|Map|IsNotEmpty (Variables|Default|GetitemsNeeded)))
      (bind _inventory (Class|BPIPlayer|GetInventory(Message) (Game|GetPlayerCharacter 0)))
      (bind _keys (Utilities|Map|Keys (Variables|Default|GetitemsNeeded)))
      (bind _array_element (Utilities|Array|ForEachLoopwithBreak _keys :!label _label)
        (:LoopBody
          (if (and (<= (- (.Value (Utilities|Map|Find (Variables|Default|GetitemsNeeded) _array_element)) 1) (.itemQuantity (Utilities|Struct|BreakS_ItemDatas (.Value (Utilities|Map|Find _inventory _array_element))))) (.ReturnValue (Utilities|Map|Find _inventory _array_element))) ; Item found ?
            (Variables|Default|SethasAllItem true)
            (else
              (Variables|Default|SethasAllItem false)
              (goto _label Break))))
        (:Completed
          (if (Variables|Default|GethasAllItem)
            (if (Variables|Default|GetuseItems)
              (bind _keys_2 (Utilities|Map|Keys (Variables|Default|GetitemsNeeded)))
              (for _array_element_2 _keys_2
                (for _index (range 0 (- (.Value (Utilities|Map|Find (Variables|Default|GetitemsNeeded) _array_element_2)) 1))
                  (Class|BPIPlayer|RemoveItemfromInventory(Message) (Game|GetPlayerCharacter 0) _array_element_2))))
            (if (Variables|Default|GetneedItemAgain)
              _
              (else
                (Variables|Default|SetneedItem false)))
            (CallFunction|InteractReaction)
            (else
              (Development|PrintString "You don't have the right item")))))
      (else
        (CallFunction|InteractReaction)))))

(event EventReact
  ;[1 0.7462 0] Trigger when an interactible object is triggered
  ; You can put the BPI Interact and override this event to make it react when an object is interacted
  (Development|PrintString (Utilities|GetDisplayName self)))

(event EventSetHighlight
  (params (Highlight :type Boolean))
  (bind _cube (Variables|Default|GetCube))
  (bind _cube_2 (Variables|Default|GetCube))
  ;[1 1 1] Highlight the interactible object
  (if Highlight
    (Rendering|SetRenderCustomDepth _cube_2 true)
    (Rendering|SetCustomDepthStencilValue _cube_2 2)
    (Class|BPIHUD|ChangeCrosshairState(Message) (HUD|GetHUD (Game|GetPlayerController 0)) true)
    (else
      (Rendering|SetRenderCustomDepth _cube false)
      (Rendering|SetCustomDepthStencilValue _cube 0)
      (Class|BPIHUD|ChangeCrosshairState(Message) (HUD|GetHUD (Game|GetPlayerController 0)) false))))

(fn ConstructionScript)