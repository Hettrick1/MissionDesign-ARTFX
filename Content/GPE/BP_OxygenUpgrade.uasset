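; BP_OxygenUpgrade is an interactable pickup that notifies the player character of an oxygen upgrade.
; On SelfReact it runs the parent reaction, disables further interaction, calls AddOxygenUpgradeMessage on the player character and plays a pickup cue.
; The actor destroys itself after a short delay plus one tick.
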(event EventSelfReact
  (|CallParentFunction)
  (Variables|Default|SetcanInterract false)
  (Class|BPIPlayer|AddOxygenUpgrade(Message) (Game|GetPlayerCharacter 0))
  (Audio|Components|Audio|Play (Variables|Default|GetPickup_Cue) 0.0)
  (Utilities|FlowControl|Delay 0.5)
  (Utilities|FlowControl|DelayUntilNextTick)
  (Actor|DestroyActor))

(fn ConstructionScript
  (|CallParentFunction))