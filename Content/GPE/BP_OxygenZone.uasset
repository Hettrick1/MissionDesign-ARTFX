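; Trigger volume that refills the player's oxygen while they stand inside its box, sized from BoxExtent in the construction script.
; BeginPlay retries each tick until the player exists, creates a paused, fast looping timer, then unpauses it if the player already overlaps.
; Box overlaps by BPI_Player actors unpause or pause that timer, which sends RefillOxygenMessage to player character 0.
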(event OnComponentBeginOverlap(Box)
  (params (OverlappedComponent :type Primitive%20Component%20Object%20Reference) (OtherActor :type Actor%20Object%20Reference) (OtherComp :type Primitive%20Component%20Object%20Reference) (OtherBodyIndex :type Integer) (bFromSweep :type Boolean) (SweepResult :type Hit%20Result%20Structure%20%28by%20ref%29))
  (if (Utilities|DoesObjectImplementInterface OtherActor "/Game/FirstPerson/Blueprints/Interface/BPI_Player.BPI_Player_C")
    (CallFunction|InfiniteOxygen)))

(event OnComponentEndOverlap(Box)
  (params (OverlappedComponent :type Primitive%20Component%20Object%20Reference) (OtherActor :type Actor%20Object%20Reference) (OtherComp :type Primitive%20Component%20Object%20Reference) (OtherBodyIndex :type Integer))
  (if (Utilities|DoesObjectImplementInterface OtherActor "/Game/FirstPerson/Blueprints/Interface/BPI_Player.BPI_Player_C")
    (Utilities|Time|PauseTimerbyHandle (Variables|Default|GettimerRef))))

(event Custom|RegenOxygen
  (Class|BPIPlayer|RefillOxygen(Message) (Game|GetPlayerCharacter 0)))

(event Custom|InfiniteOxygen
  (Utilities|Time|UnpauseTimerbyHandle (Variables|Default|GettimerRef)))

(event EventBeginPlay
  (Utilities|FlowControl|DelayUntilNextTick :!label _label)
  (Utilities|IsValid (Game|GetPlayerCharacter 0)
    (:Is%20Valid
      (bind _returnvalue (Utilities|Time|SetTimerbyEvent (delegate Custom|RegenOxygen) 0.01 true true))
      (bind _output_get (Variables|Default|SettimerRef _returnvalue))
      (Utilities|Time|PauseTimerbyHandle _output_get)
      (Utilities|FlowControl|DelayUntilNextTick)
      (Utilities|IsValid (Utilities|Array|Get(acopy) (Collision|GetOverlappingActors "/Game/FirstPerson/Blueprints/BP_FirstPersonCharacter.BP_FirstPersonCharacter_C" :!class /Script/Engine.Actor))
        (:Is%20Valid
          (CallFunction|InfiniteOxygen))))
    (:Is%20Not%20Valid
      (goto _label))))

(fn ConstructionScript
  (Components|Box|SetBoxExtent (Variables|Default|GetBox) (Variables|Default|GetboxExtent) true))