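; Trigger volume that starts a quest or completes one of its steps when its Box is overlapped.
; On overlap it calls StartQuest or UpdateQuestStep on player 0's PS_InGame, depending on NewQuest, without filtering the overlapping actor.
; The construction script looks up DT_Quests by row index to fill QuestName and StepName, clamping Step and marking optional steps.
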(event OnComponentBeginOverlap(Box)
  (params (OverlappedComponent :type Primitive%20Component%20Object%20Reference) (OtherActor :type Actor%20Object%20Reference) (OtherComp :type Primitive%20Component%20Object%20Reference) (OtherBodyIndex :type Integer) (bFromSweep :type Boolean) (SweepResult :type Hit%20Result%20Structure%20%28by%20ref%29))
  (bind _returnvalue (Game|GetPlayerState 0))
  (bind _index (Variables|Default|Getindex))
  (bind _asps_in_game (Utilities|Casting|CastToPS_InGame _returnvalue))
  (if (Variables|Default|GetnewQuest)
    (Default|StartQuest _asps_in_game _index)
    (else
      (Default|UpdateQuestStep _asps_in_game _index (Variables|Default|Getstep) true))))

(fn ConstructionScript
  (bind _outrownames (DataTable|GetDataTableRowNames "/Game/DataAssets/DT_Quests.DT_Quests"))
  (bind _returnvalue (Utilities|GetDataTableRow "/Game/DataAssets/DT_Quests.DT_Quests" (Utilities|Array|Get(acopy) _outrownames (Variables|Default|Getindex)))
    (:then
      (Variables|Default|SetquestName (.name (Utilities|Struct|BreakS_Quests _returnvalue)))
      (if (Variables|Default|GetnewQuest)
        (Variables|Default|SetstepName "disabled")
        (Variables|Default|Setstep -1)
        (else
          (Variables|Default|Setstep (Math|Integer|Clamp(Integer) (Variables|Default|Getstep) 0 (Utilities|Array|LastIndex (.queststeps (Utilities|Struct|BreakS_Quests _returnvalue)))))
          (Variables|Default|SetstepName (Utilities|String|SelectText (Utilities|Text|ToText(String) (Utilities|String|Append (Utilities|String|ToString(Text) (.name (Utilities|Struct|BreakS_Steps (Utilities|Array|Get(acopy) (.queststeps (Utilities|Struct|BreakS_Quests _returnvalue)) (Math|Integer|Clamp(Integer) (Variables|Default|Getstep) 0 (Utilities|Array|LastIndex (.queststeps (Utilities|Struct|BreakS_Quests _returnvalue)))))))) " (optional)")) (.name (Utilities|Struct|BreakS_Steps (Utilities|Array|Get(acopy) (.queststeps (Utilities|Struct|BreakS_Quests _returnvalue)) (Math|Integer|Clamp(Integer) (Variables|Default|Getstep) 0 (Utilities|Array|LastIndex (.queststeps (Utilities|Struct|BreakS_Quests _returnvalue))))))) (.optional (Utilities|Struct|BreakS_Steps (Utilities|Array|Get(acopy) (.queststeps (Utilities|Struct|BreakS_Quests _returnvalue)) (Math|Integer|Clamp(Integer) (Variables|Default|Getstep) 0 (Utilities|Array|LastIndex (.queststeps (Utilities|Struct|BreakS_Quests _returnvalue))))))))))))
    (:RowNotFound
      (Variables|Default|SetquestName "unknown")
      (Variables|Default|Setstep (Utilities|Array|LastIndex _outrownames)))))