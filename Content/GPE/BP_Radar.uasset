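; BP_Radar is a radar prop that, once its inherited SelfReact fires, reveals its antenna and starts it turning.
; Two looping timers are created paused on BeginPlay, then unpaused by SelfReact, which also plays AntennaFixed.
; The slower timer picks a random target yaw every few seconds.
; The fast timer acts as a custom tick, easing the antenna's world yaw toward that target with FInterpTo.
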(event Custom|Tick
  (bind _antenna (Variables|Default|GetAntenna))
  (bind _returnvalue (Transformation|GetWorldRotation _antenna))
  (Transformation|SetWorldRotation _antenna (Math|Rotator|MakeRotator (.roll _returnvalue) (.pitch _returnvalue) (Math|Interpolation|FInterpTo (.yaw _returnvalue) (Variables|Default|GetantennaRotation) (Utilities|Time|GetWorldDeltaSeconds) 1.0)) false false))

(event Custom|SetAntennaRotation
  (Variables|Default|SetantennaRotation (Math|Random|RandomFloatinRange -1.8e+02 1.8e+02)))

(event EventBeginPlay
  (bind _returnvalue (Utilities|Time|SetTimerbyEvent (delegate Custom|SetAntennaRotation) 3.0 true true))
  (bind _output_get (Variables|Default|SetantennaRotationTimer _returnvalue))
  (Utilities|Time|PauseTimerbyHandle _output_get)
  (bind _returnvalue_2 (Utilities|Time|SetTimerbyEvent (delegate Custom|Tick) 0.01 true true))
  (bind _output_get_2 (Variables|Default|SettickRef _returnvalue_2))
  (Utilities|Time|PauseTimerbyHandle _output_get_2))

(event EventSelfReact
  (|CallParentFunction)
  (Development|SetHiddeninGame (Variables|Default|GetAntenna) false false)
  (Utilities|Time|UnpauseTimerbyHandle (Variables|Default|GetantennaRotationTimer))
  (Utilities|Time|UnpauseTimerbyHandle (Variables|Default|GettickRef))
  (Audio|Components|Audio|Play (Variables|Default|GetAntennaFixed) 0.0))

(fn ConstructionScript
  (|CallParentFunction))