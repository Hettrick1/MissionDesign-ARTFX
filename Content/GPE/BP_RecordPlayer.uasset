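; BP_RecordPlayer is a record player gameplay element that animates when its SelfReact event fires, after running the parent's reaction.
; A timeline spins Cube1 and Cube2 through full roll turns in opposite directions at a fixed pitch.
; The timeline loops by replaying itself one tick after finishing, while a parallel sequence branch stops it after a fixed delay of a few seconds.
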(event EventSelfReact
  (|CallParentFunction)
  (Utilities|FlowControl|Sequence
    (:then_0
      (bind _newtrack_0 (Timeline|Timeline PlayFromStart)
        (:Update
          (Transformation|SetRelativeRotation (Variables|Default|GetCube2) (Math|Rotator|MakeRotator (Math|Float|Lerp 0.0 3.6e+02 _newtrack_0) 9e+01 0.0) false false)
          (Transformation|SetRelativeRotation (Variables|Default|GetCube1) (Math|Rotator|MakeRotator (* (Math|Float|Lerp 0.0 3.6e+02 _newtrack_0) -1.0) 9e+01 0.0) false false))
        (:Finished
          (Utilities|FlowControl|DelayUntilNextTick)
          (Timeline|Timeline PlayFromStart))))
    (:then_1
      (Utilities|FlowControl|Delay 7.2)
      (Timeline|Timeline Stop))))

(fn ConstructionScript
  (|CallParentFunction))