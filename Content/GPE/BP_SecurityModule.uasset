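; BP_SecurityModule is a gameplay element that advances quest index 2 each time its SelfReact event fires.
; It sets its WBP_SecurityModule widget inactive, then uses the player state's StepIndex to complete the matching step and pass a dialogue index.
; The third step also completes the quest and swaps streamed levels, unloading the normal and lockdown HQ levels and loading the security protocol level.
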(event EventSelfReact
  (bind _playerstateref (Variables|Default|GetplayerStateRef))
  (bind _aswbp_security_module (Utilities|Casting|CastToWBP_SecurityModule (UserInterface|GetWidget (Variables|Default|GetWidget))))
  (Default|SetInactive _aswbp_security_module)
  (switch int (Variables|/Game/Manager/PS_InGame.PS_InGame_C|GetstepIndex (Variables|Default|GetplayerStateRef))
    (:0
      (Default|UpdateQuestStep _playerstateref 2 1 true 10))
    (:1
      (Default|UpdateQuestStep _playerstateref 2 2 true 12))
    (:2
      (Default|UpdateQuestStep _playerstateref 2 3 true 13)
      (Default|UpdateQuestStep _playerstateref 2 0 true -1)
      (Class|GameplayStatics|UnloadStreamLevelbySoftObjectPtr "/Game/Levels/Sublevels/LVL_HQ_1Normal.LVL_HQ_1Normal" false)
      (Class|GameplayStatics|UnloadStreamLevelbySoftObjectPtr "/Game/Levels/Sublevels/LVL_HQ_2Lockdown.LVL_HQ_2Lockdown" false)
      (Class|GameplayStatics|LoadStreamLevelbySoftObjectPtr "/Game/Levels/Sublevels/LVL_HQ_3SecurityProtocole.LVL_HQ_3SecurityProtocole" true false))))

(fn ConstructionScript
  (|CallParentFunction))