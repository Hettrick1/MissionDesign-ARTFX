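; BP_SoundTrigger is a one-shot sound trigger volume that plays a configurable sound when the player enters it.
; BeginPlay assigns SoundToPlay to the Audio component.
; The first overlap by BP_FirstPersonCharacter plays it through a DoOnce, waits for the sound's duration, then destroys the actor.
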(event OnComponentBeginOverlap(TriggerSound)
  (params (OverlappedComponent :type Primitive%20Component%20Object%20Reference) (OtherActor :type Actor%20Object%20Reference) (OtherComp :type Primitive%20Component%20Object%20Reference) (OtherBodyIndex :type Integer) (bFromSweep :type Boolean) (SweepResult :type Hit%20Result%20Structure%20%28by%20ref%29))
  (Utilities|Casting|CastToBP_FirstPersonCharacter OtherActor)
  (Utilities|FlowControl|DoOnce false
    (:Completed
      (Audio|Components|Audio|Play (Variables|Default|GetAudio) 0.0)
      (Utilities|FlowControl|Delay (Variables|/Script/Engine.SoundBase|GetDuration (Variables|Default|GetsoundToPlay)))
      (Actor|DestroyActor))))

(event EventBeginPlay
  (Audio|Components|Audio|SetSound (Variables|Default|GetAudio) (Variables|Default|GetsoundToPlay)))

(fn ConstructionScript)